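; Mordhau server actor that replies to a chat command by broadcasting a Discord link as a ServerSay message.
; On BeginPlay it binds to the game mode's OnMessageBroadcasted event and loads DiscordLink from the DiscordURL custom config variable in the FTR section, if valid.
; Each broadcast is checked with MessageHasCommand, a case-insensitive prefix match credited to SoomRK, and a match triggers the reply.
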(event Custom|OnMessageBroadcasted_Event_0
  (params (Sender :type Actor%20Object%20Reference) (Msg :type String) (Type :type Name))
  (if (.ReturnValue (CallFunction|MessageHasCommand Msg (Variables|Default|GetCommand)))
    (bind _asmordhau_game_mode (Utilities|Casting|CastToMordhauGameMode (Game|GetGameMode)))
    (Class|MordhauGameMode|Broadcast _asmordhau_game_mode self (Variables|Default|GetDiscordLink) "ServerSay")))

(event EventBeginPlay
  (bind (_isvalid _returnvalue) (Class|MordhauUtilityLibrary|GetCustomConfigVarString "FTR" "DiscordURL"))
  (bind _asmordhau_game_mode (Utilities|Casting|CastToMordhauGameMode (Game|GetGameMode)))
  (EventDispatchers|AssignOnMessageBroadcasted _asmordhau_game_mode (delegate Custom|OnMessageBroadcasted_Event_0))
  (if _isvalid
    (Variables|Default|SetDiscordLink _returnvalue)))

(event Collision|EventActorBeginOverlap
  (params (OtherActor :type Actor%20Object%20Reference)))

(event EventTick
  (params (DeltaSeconds :type Float%20%28single-precision%29)))

(fn ConstructionScript)

(fn MessageHasCommand
  (params (Message :type String) (Command :type String))
  ;[1 1 1] Credit for this function goes to SoomRK. https://github.com/SoomRK/HordeStuff2
  (Variables|Default|SetMessage%20X Message)
  (Variables|Default|SetCommand%20X Command)
  (if (Utilities|String|StartsWith (Variables|Default|GetMessage%20X) (Variables|Default|GetCommand%20X))
    (return true (Utilities|String|GetSubstring (Variables|Default|GetMessage%20X) (Utilities|String|Len (Variables|Default|GetCommand%20X)) (- (Utilities|String|Len (Variables|Default|GetMessage%20X)) (Utilities|String|Len (Variables|Default|GetCommand%20X)))))
    (else
      (return false ""))))